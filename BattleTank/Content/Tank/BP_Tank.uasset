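; BP_Tank is the player-drivable tank pawn, wiring its barrel, turret and tracks into aiming and movement components on BeginPlay.
; Movement input feeds TankMovement, Fire triggers TankAiming, and aim axes rotate an azimuth gimbal and spring arm, scaled by delta time.
; A toggle action swaps between the main and first-person cameras.
; It also passes itself to its UI_HealthBar widget.
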(event EventBeginPlay
  (Class|TankAimingComponent|Initial (Variables|Default|GetTankAiming) (Variables|Default|GetTankBarrel) (Variables|Default|GetTankTurret))
  (Class|TankMovementComponent|InitialTankTrack (Variables|Default|GetTankMovement) (Variables|Default|GetLeftTrack) (Variables|Default|GetRightTrack))
  (bind _asui_health_bar (Utilities|Casting|CastToUI_HealthBar (UserInterface|GetUserWidgetObject (Variables|Default|GetHealthWidget))))
  (Variables|/Game/UI/UI_HealthBar.UI_HealthBar_C|SetTankRef _asui_health_bar self))

(event Collision|EventActorBeginOverlap
  (params (OtherActor :type Actor%20Object%20Reference)))

(event EventTick
  (params (DeltaSeconds :type Float%20%28single-precision%29)))

(event Input|ActionEvents|InputActionFire
  (params (Key :type Key%20Structure))
  ;[1 1 1] Input
  (:Pressed
    (Class|TankAimingComponent|Fire (Variables|Default|GetTankAiming))))

(event Input|ActionEvents|InputActionToggleCamera
  (params (Key :type Key%20Structure))
  ;[1 1 1] Input
  (:Pressed
    (Components|Activation|ToggleActive (Variables|Default|GetCamera))
    (Components|Activation|ToggleActive (Variables|Default|GetFirstPersonCamera))))

(event Input|AxisEvents|InputAxisAimAzimuth
  (params (AxisValue :type Float%20%28single-precision%29))
  ;[1 1 1] Input
  (Transformation|AddLocalRotation (Variables|Default|GetAzimuthGimbal) (Math|Rotator|MakeRotator 0.0 0.0 (* AxisValue (Utilities|Time|GetWorldDeltaSeconds) 1e+02)) false false))

(event Input|AxisEvents|InputAxisAimElevation
  (params (AxisValue :type Float%20%28single-precision%29))
  ;[1 1 1] Input
  (Transformation|AddLocalRotation (Variables|Default|GetSpringArm) (Math|Rotator|MakeRotator 0.0 (* AxisValue (Utilities|Time|GetWorldDeltaSeconds) 1e+02) 0.0) false false))

(event Input|AxisEvents|InputAxisMoveForward
  (params (AxisValue :type Float%20%28single-precision%29))
  ;[1 1 1] Input
  (Class|TankMovementComponent|MoveForward (Variables|Default|GetTankMovement) AxisValue))

(event Input|AxisEvents|InputAxisMoveRight
  (params (AxisValue :type Float%20%28single-precision%29))
  ;[1 1 1] Input
  (Class|TankMovementComponent|MoveRight (Variables|Default|GetTankMovement) AxisValue))

(fn ConstructionScript)